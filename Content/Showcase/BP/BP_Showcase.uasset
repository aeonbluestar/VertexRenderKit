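; BP_Showcase is an environment actor that sets up a skybox and matching post-processing look for a showcase scene.
; The construction script picks a cubemap from preset sky types or a custom override, then applies it, intensity and color to a dynamic skybox material.
; The same cubemap feeds the post-process ambient cubemap, alongside exposed exposure, fringe, vignette, grain and ambient occlusion settings.
; BeginPlay reapplies the cubemap to the material.
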(event `self.ReceiveBeginPlay`
  (`MaterialInstanceDynamic.SetTextureParameterValue` (`self.MatSkybox`) "Skybox" (`self.CubeMap`)))

(fn `UserConstructionScript`
  (bind _matskybox (`self.MatSkybox`))
  (if (== (`self.Custom Skybox`) null)
    (switch `/Game/Showcase/BP/BPE_SkyTypes` (`self.SkyType`)
      (:`NewEnumerator0`
        (set `self.CubeMap` "/Game/Showcase/HDR/Stairs.Stairs"))
      (:`NewEnumerator1`
        (set `self.CubeMap` "/Game/Showcase/HDR/Greenhouse3_Ref.Greenhouse3_Ref"))
      (:`NewEnumerator2`
        (set `self.CubeMap` "/Game/Showcase/HDR/Room.Room"))
      (:`NewEnumerator3`
        (set `self.CubeMap` "/Game/Showcase/HDR/Factory.Factory"))
      (:`NewEnumerator4`
        (set `self.CubeMap` "/Game/Showcase/HDR/Winter.Winter"))
      (:`NewEnumerator5`
        (set `self.CubeMap` "/Game/Showcase/HDR/SkatePark.SkatePark")))
    (else
      (set `self.CubeMap` (`self.Custom Skybox`))))
  (set `self.MatSkybox` null)
  (bind _returnvalue (`PrimitiveComponent.CreateDynamicMaterialInstance` 0 "/Game/Showcase/Models/MI_Skybox.MI_Skybox"))
  (set `self.MatSkybox` _returnvalue)
  (`MaterialInstanceDynamic.SetTextureParameterValue` _matskybox "Skybox" (`self.CubeMap`))
  (`MaterialInstanceDynamic.SetScalarParameterValue` _matskybox "Intensity" (`self.SkyboxIntensity`))
  (`MaterialInstanceDynamic.SetVectorParameterValue` _matskybox "SkyboxColor" (`self.SkyboxColor`))
  (set `PostProcessComponent.Settings` (make `PostProcessSettings` :`SceneFringeIntensity` (`self.Fringe`) :`Bloom5Size` 100.0 :`AmbientCubemapIntensity` (`self.HDR_Intensity`) :`AmbientCubemap` (`self.CubeMap`) :`AutoExposureBias` (`self.Exposure`) :`AutoExposureMinBrightness` 0.5 :`AutoExposureMaxBrightness` 0.75 :`LensFlareIntensity` 0.0 :`VignetteIntensity` (`self.Vignette`) :`GrainJitter` 0.2 :`GrainIntensity` (`self.GrainIntensity`) :`AmbientOcclusionIntensity` (`self.AmbientOcclusion`) :`AmbientOcclusionRadius` 40.0 :`DepthOfFieldFocalRegion` 100000.0 :`ScreenSpaceReflectionQuality` 100.0) (`self.PP`)))